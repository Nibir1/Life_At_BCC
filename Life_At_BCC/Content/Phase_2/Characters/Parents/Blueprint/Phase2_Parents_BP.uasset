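; Phase 2 parents actor that idles Mom and Dad and plays a one-time talking cutscene when the player approaches.
; Overlapping the interaction component while interaction is allowed disables player input, switches to the player's cinematic camera and loops Mom's talking animation.
; After a fixed delay it restores the main camera, Mom's idle and input, then clears the interaction flag.
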(event `self.ReceiveBeginPlay`
  (`SkeletalMeshComponent.PlayAnimation` (`self.Mom`) "/Game/Phase_2/Characters/Parents/Mom/Animation/Mom_Idle_Anim.Mom_Idle_Anim" true)
  (`SkeletalMeshComponent.PlayAnimation` (`self.Dad`) "/Game/Phase_2/Characters/Parents/Dad/Breathing_Idle.Breathing_Idle" true))

(event `self.Player_Interaction.OnComponentBeginOverlap`
  (params (OverlappedComponent :type "PrimitiveComponent Object Reference") (OtherActor :type "Actor Object Reference") (OtherComp :type "PrimitiveComponent Object Reference") (OtherBodyIndex :type Integer) (bFromSweep :type Boolean) (SweepResult :type "HitResult Structure (by ref)"))
  (bind _pjp_2_bp (`self.PJP_2_BP`))
  (bind _pjp_2_bp_2 (`self.PJP_2_BP`))
  (bind _aspjp_2_bp (cast `/Game/Phase_2/Characters/Phase_2_Player/Blueprint/PJP_2_BP` OtherActor))
  (set `self.PJP_2_BP` _aspjp_2_bp)
  (if (`self.bCan_Interact?`)
    (`self.DisableInput` _pjp_2_bp_2 (`GameplayStatics.GetPlayerController` 0))
    (`ActorComponent.Deactivate` (`/Game/Phase_2/Characters/Phase_2_Player/Blueprint/PJP_2_BP.Main_Camera` _pjp_2_bp_2))
    (`ActorComponent.Activate` (`/Game/Phase_2/Characters/Phase_2_Player/Blueprint/PJP_2_BP.Cinematic_Camera` _pjp_2_bp_2) false)
    (`SkeletalMeshComponent.PlayAnimation` (`self.Mom`) "/Game/Phase_2/Characters/Parents/Mom/Animation/Mom_Talking_Anim.Mom_Talking_Anim" true)
    (`KismetSystemLibrary.Delay` 5.167)
    (`ActorComponent.Deactivate` (`/Game/Phase_2/Characters/Phase_2_Player/Blueprint/PJP_2_BP.Cinematic_Camera` _pjp_2_bp))
    (`ActorComponent.Activate` (`/Game/Phase_2/Characters/Phase_2_Player/Blueprint/PJP_2_BP.Main_Camera` _pjp_2_bp) false)
    (`SkeletalMeshComponent.PlayAnimation` (`self.Mom`) "/Game/Phase_2/Characters/Parents/Mom/Animation/Mom_Idle_Anim.Mom_Idle_Anim" true)
    (`self.EnableInput` (`self.PJP_2_BP`) (`GameplayStatics.GetPlayerController` 0))
    (set `self.bCan_Interact?` false)))

(fn `UserConstructionScript`)