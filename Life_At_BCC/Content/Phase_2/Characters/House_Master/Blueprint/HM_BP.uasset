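; House Master NPC for Phase 2 that switches between idle and talking animations around a conversation with the player.
; When PJP_2_BP overlaps Player_Interaction, it disables that character's input, fires the IsStandingOnThePlayerInteraction dispatcher and, after a short delay, loops the talking animation.
; At BeginPlay it starts idling and binds to Phase_2_PlayerController's HouseMasterConvoDone event to resume idle.
; It does not re-enable input itself.
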(event `Start_Idle_Anim`
  (`SkeletalMeshComponent.PlayAnimation` (`self.House_Master`) "/Game/Phase_2/Characters/House_Master/Animation/HM_Idle.HM_Idle" true))

(event `self.ReceiveBeginPlay`
  (`SkeletalMeshComponent.PlayAnimation` (`self.House_Master`) "/Game/Phase_2/Characters/House_Master/Animation/HM_Idle.HM_Idle" true)
  (bind _asphase_2_player_controller (cast `/Game/Phase_2/Characters/Phase_2_Player/Blueprint/Phase_2_PlayerController` (`GameplayStatics.GetPlayerController` 0)))
  (add `/Game/Phase_2/Characters/Phase_2_Player/Blueprint/Phase_2_PlayerController.House_Master_Convo_Done` _asphase_2_player_controller (delegate `Start_Idle_Anim`)))

(event `self.Player_Interaction.OnComponentBeginOverlap`
  (params (OverlappedComponent :type "PrimitiveComponent Object Reference") (OtherActor :type "Actor Object Reference") (OtherComp :type "PrimitiveComponent Object Reference") (OtherBodyIndex :type Integer) (bFromSweep :type Boolean) (SweepResult :type "HitResult Structure (by ref)"))
  (bind _aspjp_2_bp (cast `/Game/Phase_2/Characters/Phase_2_Player/Blueprint/PJP_2_BP` OtherActor))
  (bind _output_get (set `self.PJP_2_BP` _aspjp_2_bp))
  (`self.DisableInput` _output_get (`GameplayStatics.GetPlayerController` 0))
  (`self.Is_Standing_On_The_Player_Interaction`)
  (`KismetSystemLibrary.Delay` 0.5)
  (`SkeletalMeshComponent.PlayAnimation` (`self.House_Master`) "/Game/Phase_2/Characters/House_Master/Animation/HM_Talking.HM_Talking" true))

(fn `UserConstructionScript`)