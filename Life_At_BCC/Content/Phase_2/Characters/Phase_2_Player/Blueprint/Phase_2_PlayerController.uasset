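; Player controller for Phase 2 that restores the player's saved location on startup and runs the House Master interaction UI.
; BeginPlay teleports the pawn from the "Apple" save slot, then, after delays, creates the mission and House Master widgets and caches actor and animation references.
; House Master events show its HUD with cinematic camera and cursor, and room-info completion triggers the conversation-done call.
; Escape quits the game.
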(event `Key|Escape`
  (params (Key :type "Key Structure"))
  (:`Pressed`
    (`KismetSystemLibrary.QuitGame` null "Quit")))

(event `self.ReceiveBeginPlay`
  ;[1 0.6543 0.2997] Event_Begin_Play
  ;[0.9564 0.6266 1] Teleporting_Player_To_Last_Location_And_Setting_Missions
  (`self.Teleport_Player_To_Last_Location`)
  (`KismetSystemLibrary.Delay` 1.0)
  ;[1 0.9567 0.4308] Adding_Phase2_Mission_Update_HUD_To_Viewport
  (`self.Phase2_Mission_Update_HUD_Creation`)
  (`KismetSystemLibrary.Delay` 0.5)
  (`UserWidget.AddToViewport` (`self.Phase_2_Mission_Update_HUD`) 0)
  ;[0.5637 1 0.5878] Using_The_CEV_Create_Phase2_House_Master_HUD
  (`self.Create_Phase2_House_Master_HUD`)
  ;[0.5637 1 0.5878] Using_The_CEV_Get_Phase2_House_Master_BP
  (`self.Get_House_Master_BP`)
  ;[1 1 1] Using_The_CEV_Cast_To_PJP_2_AnimBP
  (`self.Cast_To_PJP_2_AnimBP`)
  ;[0.3763 0.09336 0.3161] Binding Events Here
  (add `/Game/Phase_2/Characters/House_Master/Blueprint/HM_BP.Is_Standing_On_The_Player_Interaction` (`self.Phase_2_House_Master_BP`) (delegate `House_Master_HUD`))
  (add `/Game/HUD/Phase_2/Phase_2_House_Master_HUD.Getting_Room_Info_Finished` (`self.Phase2_House_Master_HUD`) (delegate `Getting_Room_Info_Finished`)))

(event `Cast_To_PJP_2_AnimBP`
  ;[0.5284 1 0.9502] Casting_To_PJP_2_BP_And_PJP_2_AnimBP
  (bind _aspjp_2_bp (cast `/Game/Phase_2/Characters/Phase_2_Player/Blueprint/PJP_2_BP` (`GameplayStatics.GetPlayerCharacter` 0)))
  (bind _output_get (set `self.PJP_2_BP` _aspjp_2_bp))
  (bind _aspjp_2_anim (cast `/Game/Phase_2/Characters/Phase_2_Player/Animations/PJP_2_Anim` (`SkeletalMeshComponent.GetAnimInstance` (`Character.Mesh` _output_get))))
  (set `self.PJP_2_AnimBP` _aspjp_2_anim))

(event `House_Master_HUD`
  (bind _phase2_house_master_hud (`self.Phase2_House_Master_HUD`))
  (bind _pjp_2_bp (`self.PJP_2_BP`))
  ;[0.6626 0.4247 1] Adding_Phase2_House_Master_HUD_To_Screen ( Phase 2 House Master )
  (`UserWidget.AddToViewport` _phase2_house_master_hud 0)
  (`ActorComponent.Deactivate` (`/Game/Phase_2/Characters/Phase_2_Player/Blueprint/PJP_2_BP.Main_Camera` _pjp_2_bp))
  (`ActorComponent.Activate` (`/Game/Phase_2/Characters/Phase_2_Player/Blueprint/PJP_2_BP.Cinematic_Camera` _pjp_2_bp) false)
  (`WidgetBlueprintLibrary.SetInputMode_GameAndUIEx` self _phase2_house_master_hud)
  (set `self.bShowMouseCursor` true))

(event `Phase2_Mission_Update_HUD_Creation`
  ;[0.1939 1 0.2324] Creating_Phase2_Mission_Update_HUD
  (bind _returnvalue (`|CreateWidget` "/Game/HUD/Phase_2/Phase2_Mission_Update_HUD.Phase2_Mission_Update_HUD_C"))
  (set `self.Phase_2_Mission_Update_HUD` _returnvalue))

(event `Getting_Room_Info_Finished`
  ;[0.5579 1 0.7463] Getting_Room_Info_Finished
  (`self.House_Master_Convo_Done`))

(event `Create_Phase2_House_Master_HUD`
  ;[0.7313 0.6866 1] Phase2_House_Master_HUD_Creation
  (bind _returnvalue (`|CreateWidget` "/Game/HUD/Phase_2/Phase_2_House_Master_HUD.Phase_2_House_Master_HUD_C"))
  (set `self.Phase2_House_Master_HUD` _returnvalue))

(event `Get_House_Master_BP`
  ;[0.1763 0.8701 1] Getting_Phase2_House_Master_BP
  (bind _outactors (`GameplayStatics.GetAllActorsOfClass` "/Game/Phase_2/Characters/House_Master/Blueprint/HM_BP.HM_BP_C"))
  (set `self.Phase_2_House_Master_BP` (`|GetArrayItem` _outactors)))

(fn `Teleport_Player_To_Last_Location`
  (bind _returnvalue (`GameplayStatics.LoadGameFromSlot` "Apple"))
  (bind _asmy_save_game (cast `/Game/Global_Management/Save_Game/MySaveGame` _returnvalue))
  (bind _output_get (set `self.MySaveGame` _asmy_save_game))
  (`/Engine/EditorBlueprintResources/StandardMacros.IsValid` _output_get
    (:`Is Valid`
      (`self.K2_TeleportTo` (`GameplayStatics.GetPlayerPawn` 0) (`/Game/Global_Management/Save_Game/MySaveGame.Last_Location_Save` _output_get) (`/Game/Global_Management/Save_Game/MySaveGame.Last_Rotation_Save` _output_get)))))

(fn `UserConstructionScript`)