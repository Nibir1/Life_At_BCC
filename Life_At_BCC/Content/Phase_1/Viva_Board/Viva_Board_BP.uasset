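; Viva board actor for Phase 1 that stages an oral exam by three seated panelists: Army, Civil1 and Civil2.
; Player and controller events bound on BeginPlay chain their turns, from the player sitting down through each answer finishing.
; After a short delay, each turn calls that panelist's questions, with looping animation swaps marking Army and Civil1 as speakers.
; Overlapping Viva_Notify sets HasSitForViva, cleared when the viva finishes.
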(event `Play_Idle_Anim_For_Army_Civil1_Civil2`
  ;[0.3816 1 0.4086] Play_Idle_Anim_For_Army_Civil1_Civil2_CEV_Creation
  (`SkeletalMeshComponent.PlayAnimation` (`self.Army`) "/Game/Phase_1/Characters/Army/Animations/Sitting_Idle.Sitting_Idle" true)
  (`SkeletalMeshComponent.PlayAnimation` (`self.Civil_1`) "/Game/Phase_1/Characters/Civil/Civil_1/Animations/Sitting_Idle.Sitting_Idle" true)
  (`SkeletalMeshComponent.PlayAnimation` (`self.Civil_2`) "/Game/Phase_1/Characters/Civil/Civil_2/Animations/Sitting.Sitting" true))

(event `self.ReceiveBeginPlay`
  (`self.Play_Idle_Anim_For_Army_Civil1_Civil2`)
  (bind _aspbp_1_bp (cast `/Game/Phase_1/Characters/Phase_1_Player/Blueprints/PBP_1_BP` (`GameplayStatics.GetPlayerCharacter` 0)))
  (bind _asphase_1_player_controller (cast `/Game/Phase_1/Characters/Phase_1_Player/Blueprints/Phase_1_PlayerController` (`GameplayStatics.GetPlayerController` 0)))
  (bind _output_get (set `self.Phase_1_PlayerController` _asphase_1_player_controller))
  ;[0.451 1 0.4177] Binding_Events_Here
  (add `/Game/Phase_1/Characters/Phase_1_Player/Blueprints/PBP_1_BP.Sitting_On_Chair_Viva` _aspbp_1_bp (delegate `Army_Term`))
  (add `/Game/Phase_1/Characters/Phase_1_Player/Blueprints/Phase_1_PlayerController.Army_Answering_Finished` _output_get (delegate `Civil_1_Term`))
  (add `/Game/Phase_1/Characters/Phase_1_Player/Blueprints/Phase_1_PlayerController.Civil_1_Answering_Finished` _output_get (delegate `Civil_2_Term`))
  (add `/Game/Phase_1/Characters/Phase_1_Player/Blueprints/Phase_1_PlayerController.Viva_Finished` _output_get (delegate `Reset_Has_Sit_For_Viva`)))

(event `self.Viva_Notify.OnComponentBeginOverlap`
  (params (OverlappedComponent :type "PrimitiveComponent Object Reference") (OtherActor :type "Actor Object Reference") (OtherComp :type "PrimitiveComponent Object Reference") (OtherBodyIndex :type Integer) (bFromSweep :type Boolean) (SweepResult :type "HitResult Structure (by ref)"))
  (cast `/Game/Phase_1/Characters/Phase_1_Player/Blueprints/PBP_1_BP` OtherActor)
  (set `self.Has_Sit_For_Viva` true))

(event `Army_Term`
  (`KismetSystemLibrary.Delay` 0.6)
  (`SkeletalMeshComponent.PlayAnimation` (`self.Army`) "/Game/Phase_1/Characters/Army/Animations/Having_A_Meeting__Male.Having_A_Meeting__Male" true)
  (`self.Army_Asking_Questions`))

(event `Civil_1_Term`
  (`KismetSystemLibrary.Delay` 0.6)
  (`SkeletalMeshComponent.PlayAnimation` (`self.Army`) "/Game/Phase_1/Characters/Army/Animations/Sitting_Idle.Sitting_Idle" true)
  (`SkeletalMeshComponent.PlayAnimation` (`self.Civil_1`) "/Game/Phase_1/Characters/Civil/Civil_1/Animations/Having_A_Meeting__Male.Having_A_Meeting__Male" true)
  (`self.Civil_1_Asking_Questions`))

(event `Civil_2_Term`
  (`KismetSystemLibrary.Delay` 0.6)
  (`SkeletalMeshComponent.PlayAnimation` (`self.Civil_1`) "/Game/Phase_1/Characters/Civil/Civil_1/Animations/Sitting_Idle.Sitting_Idle" true)
  (`self.Civil_2_Asking_Questions`))

(event `Reset_Has_Sit_For_Viva`
  (set `self.Has_Sit_For_Viva` false))

(fn `UserConstructionScript`)