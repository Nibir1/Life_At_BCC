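; Phase 1 player controller that runs the exam, medical check-up and viva board stages of an admission sequence, ending in a result screen.
; BeginPlay teleports the pawn to its saved location, creates the stage widgets and finds the Teacher, Doctor and Viva Board actors.
; Bound dispatchers show each question HUD with mouse input, then relay completion, reset sitting animation flags or switch to the cinematic camera.
; Escape quits the game.
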(event `Key|Escape`
  (params (Key :type "Key Structure"))
  (:`Pressed`
    (`KismetSystemLibrary.QuitGame` null "Quit")))

(event `self.ReceiveBeginPlay`
  ;[1 0.6543 0.2997] Event_Begin_Play
  ;[0.9564 0.6266 1] Teleporting_Player_To_Last_Location_And_Setting_Missions
  (`self.Teleport_Player_To_Last_Location`)
  (`KismetSystemLibrary.Delay` 1.0)
  ;[1 0.9567 0.4308] Adding_Phase1_Mission_Update_HUD_To_Viewport
  (`self.Mission_Update_HUD_Creation`)
  (`UserWidget.AddToViewport` (`self.Phase_1_Mission_Update_HUD`) 0)
  ;[0.8294 1 0.4586] Using_The_CEV_Cast_To_Anim_BP
  (`self.Cast_To_Anim_BP`)
  ;[0.5415 1 0.9901] Using_The_CEV_Get_Doctor_BP
  (`self.Get_Doctor_BP`)
  ;[1 0.6936 0.8739] Using_The_CEV_Create_Question_Paper_HUD
  (`self.Create_Question_Paper_HUD`)
  ;[0.3228 0.9901 1] Using_The_CEV_Create_Medical_CheckUp_HUD
  (`self.Create_Medical_Checkup_HUD`)
  ;[1 0.5659 0.7848] Using_The_CEV_Get_Viva_Board_BP
  (`self.Get_Viva_Board_BP`)
  ;[1 0.9001 0.3184] Using_The_CEV_Army_Asking_HUD
  (`self.Create_Army_Asking_HUD`)
  ;[0.9194 0.3694 1] Using_The_CEV_Create_Civil1_Asking_HUD
  (`self.Create_Civil1_Asking_HUID`)
  ;[1 0.8659 0.3512] Using_The_CEV_Civil2_Asking_HUD
  (`self.Create_Civil2_Asking_HUD`)
  ;[0.6452 0.9801 1] Using_The_CEV_Get_Teacher_BP
  (`self.Get_Teacher_BP`)
  ;[1 0.2424 0.4752] Binding_Events_Here
  (add `/Game/Phase_1/Characters/Teacher/Blueprints/Teacher_BP.Teacher_Briefing` (`self.Teacher_BP`) (delegate `Question_Paper_HUD`))
  (add `/Game/HUD/Phase_1/Question_Paper_HUD.Exam_Finished` (`self.Question_Paper_HUD!`) (delegate `Get_Up_After_Exam_Finished`))
  (add `/Game/Phase_1/Characters/Doctor/Blueprint/Doctor_BP.Is_Standing_On_The_CheckUp` (`self.Doctor_BP`) (delegate `Add_Medical_CheckUp_Question_HUD`))
  (add `/Game/HUD/Phase_1/Medical_CheckUp_HUD.Medical_Check_Up_Finished` (`self.Medical_CheckUp_HUD`) (delegate `Check_Up_Finished`))
  (add `/Game/Phase_1/Viva_Board/Viva_Board_BP.Army_Asking_Questions` (`self.Viva_Board_BP`) (delegate `Add_Army_Asking_Question_HUD`))
  (add `/Game/HUD/Phase_1/Army_Asking_HUD.Army_Answering_Done_HUD` (`self.Army_Asking_HUD`) (delegate `Notify_Army_At_Viva_Board`))
  (add `/Game/Phase_1/Viva_Board/Viva_Board_BP.Civil_1_Asking_Questions` (`self.Viva_Board_BP`) (delegate `Add_Civil_1_Asking_Question_HUD`))
  (add `/Game/HUD/Phase_1/Civil_1_Asking_HUD.Civil_1_Answering_Done_HUD` (`self.Civil_1_Asking_HUD`) (delegate `Notify_Civil_1_At_Viva_Board`))
  (add `/Game/Phase_1/Viva_Board/Viva_Board_BP.Civil_2_Asking_Questions` (`self.Viva_Board_BP`) (delegate `Add_Civil_2_Asking_Question_HUD`))
  (add `/Game/HUD/Phase_1/Civil_2_Asking_HUD.Civil_2_Answering_Done_HUD` (`self.Civil_2_Asking_HUD`) (delegate `Notify_Civil_2_At_Viva_Board`)))

(event `Get_Teacher_BP`
  ;[0.5927 0.4055 1] Getting_Teacher_BP
  (bind _outactors (`GameplayStatics.GetAllActorsOfClass` "/Game/Phase_1/Characters/Teacher/Blueprints/Teacher_BP.Teacher_BP_C"))
  (set `self.Teacher_BP` (`|GetArrayItem` _outactors)))

(event `Mission_Update_HUD_Creation`
  ;[0.1939 1 0.2324] Creating_Mission_Update_HUD
  (bind _returnvalue (`|CreateWidget` "/Game/HUD/Phase_1/Phase1_Mission_Update_HUD.Phase1_Mission_Update_HUD_C"))
  (set `self.Phase_1_Mission_Update_HUD` _returnvalue))

(event `Cast_To_Anim_BP`
  ;[0.1161 1 0.8802] Casting_To_Anim_BP
  (bind _aspbp_1_bp (cast `/Game/Phase_1/Characters/Phase_1_Player/Blueprints/PBP_1_BP` (`GameplayStatics.GetPlayerCharacter` 0)))
  (bind _output_get (set `self.My_Player_BP` _aspbp_1_bp))
  (bind _aspbp_1_anim (cast `/Game/Phase_1/Characters/Phase_1_Player/Animations/PBP_1_Anim` (`SkeletalMeshComponent.GetAnimInstance` (`Character.Mesh` _output_get))))
  (set `self.My_Anim_BP` _aspbp_1_anim))

(event `Get_Doctor_BP`
  ;[1 0.2699 0.4407] Getting_Doctor_BP
  (bind _outactors (`GameplayStatics.GetAllActorsOfClass` "/Game/Phase_1/Characters/Doctor/Blueprint/Doctor_BP.Doctor_BP_C"))
  (set `self.Doctor_BP` (`|GetArrayItem` _outactors)))

(event `Question_Paper_HUD`
  (bind _question_paper_hud_ (`self.Question_Paper_HUD!`))
  ;[0.4567 0.4791 1] Adding_Question_Paper_HUD_To_Screen  ( Exam_Board )
  (`UserWidget.AddToViewport` _question_paper_hud_ 0)
  (`self.EnableInput` null)
  (`WidgetBlueprintLibrary.SetInputMode_GameAndUIEx` self _question_paper_hud_)
  (set `self.bShowMouseCursor` true))

(event `Create_Question_Paper_HUD`
  ;[0.3926 0.6865 1] Question_Paper_HUD_Creation
  (bind _returnvalue (`|CreateWidget` "/Game/HUD/Phase_1/Question_Paper_HUD.Question_Paper_HUD_C"))
  (set `self.Question_Paper_HUD!` _returnvalue))

(event `Get_Up_After_Exam_Finished`
  (bind _my_anim_bp (`self.My_Anim_BP`))
  ;[1 0.498 0.2753] Get_Up_After_Exam_Finished ( Exam_Board )
  (set `/Game/Phase_1/Characters/Phase_1_Player/Animations/PBP_1_Anim.Sitting_Idle_Chair?` false _my_anim_bp)
  (set `/Game/Phase_1/Characters/Phase_1_Player/Animations/PBP_1_Anim.Stand_To_Sit?` false _my_anim_bp)
  (set `/Game/Phase_1/Characters/Phase_1_Player/Animations/PBP_1_Anim.Sit_To_Stand?` false _my_anim_bp)
  (`self.Exam_Finished`)
  ;[0.3957 1 0.455] Hiding_Mission_2_Here
  (`/Game/HUD/Phase_1/Phase1_Mission_Update_HUD.Hide_Mission2` (`self.Phase_1_Mission_Update_HUD`)))

(event `Create_Medical_Checkup_HUD`
  ;[1 0.6905 0.5487] Medical_CheckUp_HUD_Creation
  (bind _returnvalue (`|CreateWidget` "/Game/HUD/Phase_1/Medical_CheckUp_HUD.Medical_CheckUp_HUD_C"))
  (set `self.Medical_CheckUp_HUD` _returnvalue))

(event `Add_Medical_CheckUp_Question_HUD`
  (bind _medical_checkup_hud (`self.Medical_CheckUp_HUD`))
  (bind _my_player_bp (`self.My_Player_BP`))
  ;[0.4567 0.4791 1] Adding_Medical_CheckUp_HUD_To_Screen ( Medical_Board )
  (`UserWidget.AddToViewport` _medical_checkup_hud 0)
  (`ActorComponent.Deactivate` (`/Game/Phase_1/Characters/Phase_1_Player/Blueprints/PBP_1_BP.Main_Camera` _my_player_bp))
  (`ActorComponent.Activate` (`/Game/Phase_1/Characters/Phase_1_Player/Blueprints/PBP_1_BP.Cinematic_Camera` _my_player_bp) false)
  (`WidgetBlueprintLibrary.SetInputMode_GameAndUIEx` self _medical_checkup_hud)
  (set `self.bShowMouseCursor` true))

(event `Get_Viva_Board_BP`
  ;[0.4294 1 0.7963] Getting_Viva_Board_BP
  (bind _outactors (`GameplayStatics.GetAllActorsOfClass` "/Game/Phase_1/Viva_Board/Viva_Board_BP.Viva_Board_BP_C"))
  (set `self.Viva_Board_BP` (`|GetArrayItem` _outactors)))

(event `Check_Up_Finished`
  ;[0.5579 1 0.7463] CheckUp_Finished ( Medical_Board )
  (`self.CheckUp_Finished`))

(event `Create_Army_Asking_HUD`
  ;[0 0.8346 1] Army_Asking_HUD_Creation
  (bind _returnvalue (`|CreateWidget` "/Game/HUD/Phase_1/Army_Asking_HUD.Army_Asking_HUD_C"))
  (set `self.Army_Asking_HUD` _returnvalue))

(event `Add_Army_Asking_Question_HUD`
  (bind _army_asking_hud (`self.Army_Asking_HUD`))
  ;[1 0.8886 0.3571] Adding_Army_Asking_Question_HUD_To_Screen
  (`UserWidget.AddToViewport` _army_asking_hud 0)
  (`WidgetBlueprintLibrary.SetInputMode_GameAndUIEx` self _army_asking_hud)
  (set `self.bShowMouseCursor` true))

(event `Create_Civil1_Asking_HUID`
  ;[0.3105 1 0.6903] Civil_1_Asking_HUD_Creation
  (bind _returnvalue (`|CreateWidget` "/Game/HUD/Phase_1/Civil_1_Asking_HUD.Civil_1_Asking_HUD_C"))
  (set `self.Civil_1_Asking_HUD` _returnvalue))

(event `Notify_Army_At_Viva_Board`
  ;[0.1779 0.6939 1] Notifying_Viva_Board_That_Army_Answering_Is_Done
  (`self.Army_Answering_Finished`))

(event `Create_Civil2_Asking_HUD`
  ;[0.8283 0.4362 1] Civil_2_Asking_HUD_Creation
  (bind _returnvalue (`|CreateWidget` "/Game/HUD/Phase_1/Civil_2_Asking_HUD.Civil_2_Asking_HUD_C"))
  (set `self.Civil_2_Asking_HUD` _returnvalue))

(event `Add_Civil_1_Asking_Question_HUD`
  (bind _civil_1_asking_hud (`self.Civil_1_Asking_HUD`))
  ;[1 0.6413 0.1882] Adding_Civil_1_Asking_HUD_To_Screen
  (`UserWidget.AddToViewport` _civil_1_asking_hud 0)
  (`WidgetBlueprintLibrary.SetInputMode_GameAndUIEx` self _civil_1_asking_hud)
  (set `self.bShowMouseCursor` true))

(event `Notify_Civil_1_At_Viva_Board`
  ;[1 0.1973 0.2272] Notifying_Viva_Board_That_Civil_1_Answering_Done
  (`self.Civil_1_Answering_Finished`))

(event `Add_Civil_2_Asking_Question_HUD`
  ;[0.3369 1 0.2919] Adding_Civil_2_Asking_HUD_To_Screen
  (`UserWidget.AddToViewport` (`self.Civil_2_Asking_HUD`) 0)
  (`WidgetBlueprintLibrary.SetInputMode_GameAndUIEx` self null)
  (set `self.bShowMouseCursor` true))

(event `Stand_Up_After_Viva_Finishes`
  (bind _my_anim_bp (`self.My_Anim_BP`))
  ;[0.9953 1 0.7622] Stand_Up_After_Viva_Finishes_CEV_Creation
  (set `/Game/Phase_1/Characters/Phase_1_Player/Animations/PBP_1_Anim.Sitting_Idle_Chair?` false _my_anim_bp)
  (set `/Game/Phase_1/Characters/Phase_1_Player/Animations/PBP_1_Anim.Stand_To_Sit?` false _my_anim_bp)
  (set `/Game/Phase_1/Characters/Phase_1_Player/Animations/PBP_1_Anim.Sit_To_Stand?` false _my_anim_bp))

(event `Notify_Civil_2_At_Viva_Board`
  ;[0 0.7684 1] Getting_Up_After_Viva_Finished ( Viva_Board )
  (`self.Stand_Up_After_Viva_Finishes`)
  (`self.Viva_Finished`)
  ;[1 0.8084 0.4875] Adding_Admission_Result_HUD_To_Viewport
  (`KismetSystemLibrary.Delay` 1.0)
  (`self.Create_Admission_Result_HUD`)
  (`UserWidget.AddToViewport` (`self.Admission_Result_HUD`) 0))

(event `Create_Admission_Result_HUD`
  ;[0.986 0.5993 1] Admission_Result_HUD_Creation
  (bind _returnvalue (`|CreateWidget` "/Game/HUD/Phase_1/Admission_Result_HUD.Admission_Result_HUD_C"))
  (set `self.Admission_Result_HUD` _returnvalue))

(fn `Get_Save_Game_System`
  (bind _returnvalue (`GameplayStatics.DoesSaveGameExist` "Apple"))
  (if _returnvalue
    (bind _returnvalue_2 (`GameplayStatics.LoadGameFromSlot` "Apple"))
    (bind _asmy_save_game (cast `/Game/Global_Management/Save_Game/MySaveGame` _returnvalue_2))
    (set `self.MySaveGame` _asmy_save_game)
    (else
      (bind _returnvalue_3 (`GameplayStatics.CreateSaveGameObject` "/Game/Global_Management/Save_Game/MySaveGame.MySaveGame_C"))
      (bind _asmy_save_game_2 (cast `/Game/Global_Management/Save_Game/MySaveGame` _returnvalue_3))
      (set `self.MySaveGame` _asmy_save_game_2))))

(fn `Teleport_Player_To_Last_Location`
  (bind _returnvalue (`GameplayStatics.LoadGameFromSlot` "Apple"))
  (bind _asmy_save_game (cast `/Game/Global_Management/Save_Game/MySaveGame` _returnvalue))
  (bind _output_get (set `self.MySaveGame` _asmy_save_game))
  (`/Engine/EditorBlueprintResources/StandardMacros.IsValid` _output_get
    (:`Is Valid`
      (`self.K2_TeleportTo` (`GameplayStatics.GetPlayerPawn` 0) (`/Game/Global_Management/Save_Game/MySaveGame.Last_Location_Save` _output_get) (`/Game/Global_Management/Save_Game/MySaveGame.Last_Rotation_Save` _output_get)))))

(fn `UserConstructionScript`)