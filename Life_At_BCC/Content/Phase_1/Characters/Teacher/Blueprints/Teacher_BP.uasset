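; Teacher NPC for Phase 1 that plays a timed talking sequence when the player sits on the exam chair.
; On BeginPlay it loops a breathing idle, finds the first player Blueprint actor and binds Start_Talking to its sitting event.
; After a short delay, Start_Talking loops the talking animation, fires the TeacherBriefing call midway, then returns to idle, all timed with fixed delays.
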(event `self.ReceiveBeginPlay`
  (`SkeletalMeshComponent.PlayAnimation` (`self.Mesh`) "/Game/Phase_1/Characters/Teacher/Animations/Breathing_Idle.Breathing_Idle" true)
  (bind _asteacher_bp (`self.Get_Player_BP`))
  (add `/Game/Phase_1/Characters/Phase_1_Player/Blueprints/PBP_1_BP.Sitting_On_Chair_Exam` _asteacher_bp (delegate `Start_Talking`)))

(event `Start_Talking`
  (`KismetSystemLibrary.Delay` 1.0)
  (`SkeletalMeshComponent.PlayAnimation` (`self.Mesh`) "/Game/Phase_1/Characters/Teacher/Animations/Talking.Talking" true)
  (`KismetSystemLibrary.Delay` 10.267)
  (`self.Teacher_Briefing`)
  (`KismetSystemLibrary.Delay` 10.267)
  (`SkeletalMeshComponent.PlayAnimation` (`self.Mesh`) "/Game/Phase_1/Characters/Teacher/Animations/Breathing_Idle.Breathing_Idle" true))

(fn `Get_Player_BP`
  (returns (AsTeacher_BP :type "/Game/Phase_1/Characters/Phase_1_Player/Blueprints/PBP_1_BP Object Reference"))
  (bind _outactors (`GameplayStatics.GetAllActorsOfClass` "/Game/Phase_1/Characters/Phase_1_Player/Blueprints/PBP_1_BP.PBP_1_BP_C"))
  (return (`|GetArrayItem` _outactors)))

(fn `UserConstructionScript`)