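; Phase 1 guard NPC that stops the player for a check and locks a gate once the player has passed.
; Overlapping the guard box freezes player movement, plays a talking animation, then reveals debug text and returns to idle.
; The player's GuardCheckingDone dispatcher restores walking.
; The player's first exit from the gate box plays the lock animation after a short delay and hides the first mission on the HUD.
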(event `self.ReceiveBeginPlay`
  (`SkeletalMeshComponent.PlayAnimation` (`self.Mesh`) "/Game/Phase_1/Characters/Guards/Guard_1/Animations/Breathing_Idle.Breathing_Idle" true)
  (bind _asphase_1_player_controller (cast `/Game/Phase_1/Characters/Phase_1_Player/Blueprints/Phase_1_PlayerController` (`GameplayStatics.GetPlayerController` 0)))
  (set `self.Phase1_PlayerController` _asphase_1_player_controller)
  (bind _aspbp_1_bp (cast `/Game/Phase_1/Characters/Phase_1_Player/Blueprints/PBP_1_BP` (`GameplayStatics.GetPlayerCharacter` 0)))
  (bind _output_get (set `self.PBP_1_BP` _aspbp_1_bp))
  (add `/Game/Phase_1/Characters/Phase_1_Player/Blueprints/PBP_1_BP.Guard_Checking_Done` _output_get (delegate `Activate_Players_Movement`)))

(event `self.Guard_Collision.OnComponentBeginOverlap`
  (params (OverlappedComponent :type "PrimitiveComponent Object Reference") (OtherActor :type "Actor Object Reference") (OtherComp :type "PrimitiveComponent Object Reference") (OtherBodyIndex :type Integer) (bFromSweep :type Boolean) (SweepResult :type "HitResult Structure (by ref)"))
  (cast `/Game/Phase_1/Characters/Phase_1_Player/Blueprints/PBP_1_BP` OtherActor)
  (set `self.Has_Touched_The_Guard_Box` true)
  (`self.Deactivate_Players_Movement`)
  (`SkeletalMeshComponent.PlayAnimation` (`self.Mesh`) "/Game/Phase_1/Characters/Guards/Guard_1/Animations/Talking.Talking" false)
  (`KismetSystemLibrary.Delay` 3.933)
  ;[1 0.1513 0.0916] For Debug Purpose
  (`SceneComponent.SetVisibility` (`self.TextRender`) true false)
  (`SkeletalMeshComponent.PlayAnimation` (`self.Mesh`) "/Game/Phase_1/Characters/Guards/Guard_1/Animations/Breathing_Idle.Breathing_Idle" true))

(event `self.Gate_Collision.OnComponentEndOverlap`
  (params (OverlappedComponent :type "PrimitiveComponent Object Reference") (OtherActor :type "Actor Object Reference") (OtherComp :type "PrimitiveComponent Object Reference") (OtherBodyIndex :type Integer))
  (cast `/Game/Phase_1/Characters/Phase_1_Player/Blueprints/PBP_1_BP` OtherActor)
  (`/Engine/EditorBlueprintResources/StandardMacros.DoOnce` false
    (:`Completed`
      (`KismetSystemLibrary.Delay` 1.0)
      (`SkeletalMeshComponent.PlayAnimation` (`self.Gate_Lock`) "/Game/Phase_1/Props/Gate/Gate_Lock.Gate_Lock" false)
      (`/Game/HUD/Phase_1/Phase1_Mission_Update_HUD.Hide_Mission1` (`/Game/Phase_1/Characters/Phase_1_Player/Blueprints/Phase_1_PlayerController.Phase_1_Mission_Update_HUD` (`self.Phase1_PlayerController`))))))

(event `self.Guard_Collision.OnComponentEndOverlap`
  (params (OverlappedComponent :type "PrimitiveComponent Object Reference") (OtherActor :type "Actor Object Reference") (OtherComp :type "PrimitiveComponent Object Reference") (OtherBodyIndex :type Integer))
  (cast `/Game/Phase_1/Characters/Phase_1_Player/Blueprints/PBP_1_BP` OtherActor)
  (set `self.Has_Touched_The_Guard_Box` false))

(event `Activate_Players_Movement`
  (`CharacterMovementComponent.SetMovementMode` (`Character.CharacterMovement` (`self.PBP_1_BP`)) "MOVE_Walking" 0))

(fn `Deactivate_Players_Movement`
  (`CharacterMovementComponent.SetMovementMode` (`Character.CharacterMovement` (`self.PBP_1_BP`)) "MOVE_None" 0))

(fn `UserConstructionScript`)