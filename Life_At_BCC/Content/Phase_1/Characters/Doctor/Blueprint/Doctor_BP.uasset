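; Doctor NPC for Phase 1 that runs a check-up on the player character (PBP_1_BP).
; It loops a breathing idle; entering CheckUp_Col disables player input, calls IsStandingOnTheCheckUp and, after a short delay, loops a petting animation.
; The Phase 1 player controller's CheckUpFinished binding returns the doctor to idle.
; The Doc_Notify_Col overlap only casts the other actor and has no further effect.
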(event `Start_Idle_Anim`
  (`SkeletalMeshComponent.PlayAnimation` (`self.Mesh`) "/Game/Phase_1/Characters/Doctor/Animation/Breathing_Idle.Breathing_Idle" true))

(event `self.ReceiveBeginPlay`
  (`SkeletalMeshComponent.PlayAnimation` (`self.Mesh`) "/Game/Phase_1/Characters/Doctor/Animation/Breathing_Idle.Breathing_Idle" true)
  (bind _asphase_1_player_controller (cast `/Game/Phase_1/Characters/Phase_1_Player/Blueprints/Phase_1_PlayerController` (`GameplayStatics.GetPlayerController` 0)))
  (add `/Game/Phase_1/Characters/Phase_1_Player/Blueprints/Phase_1_PlayerController.CheckUp_Finished` _asphase_1_player_controller (delegate `Start_Idle_Anim`)))

(event `self.Doc_Notify_Col.OnComponentBeginOverlap`
  (params (OverlappedComponent :type "PrimitiveComponent Object Reference") (OtherActor :type "Actor Object Reference") (OtherComp :type "PrimitiveComponent Object Reference") (OtherBodyIndex :type Integer) (bFromSweep :type Boolean) (SweepResult :type "HitResult Structure (by ref)"))
  (cast `/Game/Phase_1/Characters/Phase_1_Player/Blueprints/PBP_1_BP` OtherActor))

(event `self.CheckUp_Col.OnComponentBeginOverlap`
  (params (OverlappedComponent :type "PrimitiveComponent Object Reference") (OtherActor :type "Actor Object Reference") (OtherComp :type "PrimitiveComponent Object Reference") (OtherBodyIndex :type Integer) (bFromSweep :type Boolean) (SweepResult :type "HitResult Structure (by ref)"))
  (bind _aspbp_1_bp (cast `/Game/Phase_1/Characters/Phase_1_Player/Blueprints/PBP_1_BP` OtherActor))
  (`self.DisableInput` _aspbp_1_bp (`GameplayStatics.GetPlayerController` 0))
  (`self.Is_Standing_On_The_CheckUp`)
  (`KismetSystemLibrary.Delay` 0.5)
  (`SkeletalMeshComponent.PlayAnimation` (`self.Mesh`) "/Game/Phase_1/Characters/Doctor/Animation/Petting.Petting" true))

(fn `UserConstructionScript`)